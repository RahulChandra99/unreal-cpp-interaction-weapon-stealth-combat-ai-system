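; BP_CoinProjectile is a coin variant of a parent projectile that makes an audible noise where it explodes.
; On BeginPlay it runs the parent logic, then sets a one-second explosion time and flags itself as a coin.
; The ExplodeBP event plays the impact sound and calls MakeNoise at the coin's location, with player character 0 as instigator.
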(event `self.ReceiveBeginPlay`
  (`parent.ReceiveBeginPlay`)
  (set `self.ExplosionTime` 1.0)
  (set `self.bIsForCoin` true))

(event `self.ExplodeBP`
  (params (HitEnemies :type "Array of Actor Object Reference (by ref)"))
  (bind _returnvalue (`GameplayStatics.GetPlayerCharacter` 0))
  (`GameplayStatics.PlaySoundAtLocation` (`self.ImpactSFX`) (`self.K2_GetActorLocation`) (struct) 1.0 1.0 0.0 null null null null)
  (`self.MakeNoise` _returnvalue 1.0 _returnvalue (`self.K2_GetActorLocation`) 0.0 "None"))

(fn `UserConstructionScript`
  (`parent.UserConstructionScript`))