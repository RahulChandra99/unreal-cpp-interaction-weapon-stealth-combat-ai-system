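; BP_BaseProjectile is a base projectile actor configured by data from DT_ProjectileType.
; On BeginPlay it looks up the row named by ProjectileName, then sets movement speed and gravity, assigns the Niagara visual and plays the projectile sound at its location.
; It also stores the impact effect, impact sound and throwable flag, and zeroes Damage rather than reading it from the row.
; No hit handling is present in these graphs.
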(event `self.ReceiveBeginPlay`
  (bind _projectilemovement (`self.ProjectileMovement`))
  (bind _returnvalue (`|GetDataTableRow` "/Game/_DEV/DataTable/Abilties/DT_ProjectileType.DT_ProjectileType" (`self.ProjectileName`))
    (:`then`
      (set `ProjectileMovementComponent.InitialSpeed` (`.ProjectileSpeed_47_4290B55B498DAD74D41191A859D569F3` (break `/Game/_DEV/DataTable/Abilties/S_ProjectileType` _returnvalue)) _projectilemovement)
      (set `ProjectileMovementComponent.ProjectileGravityScale` (`.Gravity_49_480466B148EC104FCB30558F26E8F6A9` (break `/Game/_DEV/DataTable/Abilties/S_ProjectileType` _returnvalue)) _projectilemovement)
      (set `ProjectileMovementComponent.MaxSpeed` (`.ProjectileSpeed_47_4290B55B498DAD74D41191A859D569F3` (break `/Game/_DEV/DataTable/Abilties/S_ProjectileType` _returnvalue)) _projectilemovement)
      (set `self.Damage` 0.0)
      (`NiagaraComponent.SetAsset` (`self.ProjectileNS`) (`.ProjectileNS_60_4BDDA3BD4A76C59977A73784B7BF1DA3` (break `/Game/_DEV/DataTable/Abilties/S_ProjectileType` _returnvalue)) true)
      (set `self.ImpactEffect` (`.HitImpactNS_35_A8172D9C439C906EBFCB3CBE4622706F` (break `/Game/_DEV/DataTable/Abilties/S_ProjectileType` _returnvalue)))
      (set `self.ImpactSFX` (`.ImpactSFX_40_E637102A42DA0B0E20165A940DB0EFCE` (break `/Game/_DEV/DataTable/Abilties/S_ProjectileType` _returnvalue)))
      (`GameplayStatics.PlaySoundAtLocation` (`.ProjectileSFX_38_4BA1234F4CCF113171689D9750B41346` (break `/Game/_DEV/DataTable/Abilties/S_ProjectileType` _returnvalue)) (`self.K2_GetActorLocation`) (struct) 1.0 1.0 0.0 null null null null)
      (set `self.bIsProjectileThrowable` (`.IsProjectileThrowable_63_259249B84A2FCEE40700CC83576DC104` (break `/Game/_DEV/DataTable/Abilties/S_ProjectileType` _returnvalue))))))

(fn `UserConstructionScript`)