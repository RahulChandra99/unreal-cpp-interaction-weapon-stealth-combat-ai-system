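; BP_GrenadeProjectile is a grenade projectile Blueprint that provides the explosion effects and sets the timing value.
; BeginPlay calls the parent, then sets ExplosionTime.
; The ExplodeBP event spawns the impact effect sized by ExplosionScale, plays the impact sound at the grenade's location and destroys the actor.
; Nothing here calls ExplodeBP or applies damage, and the node deriving ExplosionRadius from ExplosionScale is disconnected.
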(event `self.ReceiveBeginPlay`
  (`parent.ReceiveBeginPlay`)
  (set `self.ExplosionTime` 1.0))

(event `self.ExplodeBP`
  (params (HitEnemies :type "Array of Actor Object Reference (by ref)"))
  (bind _returnvalue (`self.K2_GetActorLocation`))
  (`NiagaraFunctionLibrary.SpawnSystemAtLocation` (`self.ImpactEffect`) _returnvalue (struct) (`KismetMathLibrary.Conv_DoubleToVector` (`self.ExplosionScale`)))
  (`GameplayStatics.PlaySoundAtLocation` (`self.ImpactSFX`) _returnvalue (struct) 1.0 1.0 0.0 null null null null)
  (`self.K2_DestroyActor`))

(fn `UserConstructionScript`
  (`parent.UserConstructionScript`))