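; Player component for a stealth game that handles interactions with doors, pickups, luggage and dead enemies.
; Capsule overlaps track interactables in range and show a screen-space prompt on the latest one.
; IA_Interact acts by interaction type through montage notifies, with pickup animations chosen by a traced height above ground.
; Dead bodies open a radial wheel to loot, drag or disguise, swapping meshes and spawning a backpack of old clothes.
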(event `self.ReceiveBeginPlay`
  ;[0.7999 0.8475 1] Begin
  (bind _ascharacter (cast `Character` (`self.GetOwner`)))
  (bind _output_get (set `self.CharacterRef` _ascharacter))
  (bind _playerref (message `/Game/_DEV/Interfaces/BPI_GetCombatCharacter.GetPlayerRef` _output_get))
  (set `self.Player Ref` _playerref)
  (bind _capsulecomponent (`Character.CapsuleComponent` _ascharacter))
  (add `PrimitiveComponent.OnComponentBeginOverlap` _capsulecomponent (`|CreateDelegate` :!event `HandleBeginOverlap`))
  (add `PrimitiveComponent.OnComponentEndOverlap` _capsulecomponent (`|CreateDelegate` :!event `HandleEndOverlap`))
  (bind _returnvalue (`|AddComponentByClass` :`self` (`self.GetOwner`) :`Class` "/Script/UMG.WidgetComponent" :`bManualAttachment` true))
  (`WidgetComponent.SetWidgetSpace` _returnvalue "Screen")
  (`WidgetComponent.SetDrawSize` _returnvalue (250.0 30.0))
  (set `self.InteractionWidgetComponent` _returnvalue)
  (bind _playerref_2 (message `/Game/_DEV/Interfaces/BPI_GetCombatCharacter.GetPlayerRef` (`self.CharacterRef`)))
  (set `self.Interactions Radial Wheel` (`/Game/_DEV/Blueprints/BP_CombatCharacter.Interactions_RadialWheel` _playerref_2)))

(event `DragBody`
  ;[0.7999 0.8475 1] Drag Body
  (if (not (`self.bIsDraggingEnemy`))
    (bind _playerref (message `/Game/_DEV/Interfaces/BPI_GetCombatCharacter.GetPlayerRef` (`self.CharacterRef`)))
    (bind _enemyref (message `/Game/_DEV/Blueprints/Enemy/AI/BPI_EnemyAI.GetEnemyRef` (`self.F_GetActiveInteractable`)))
    (if (`/Game/_DEV/DamageSystem/BPC_DamageSystem.IsDead` (`/Game/_DEV/Blueprints/Enemy/BP_Enemy.BPC_DamageSystem` _enemyref))
      (`CombatProjectCharacter.GrabEnemy` _playerref _enemyref)
      (set `self.bIsDraggingEnemy` true)
      (set `CombatProjectCharacter.bIsCrouching` true _playerref)
      (set `CharacterMovementComponent.MaxWalkSpeed` (`/Game/_DEV/Blueprints/BP_CombatCharacter.CrouchSpeed` _playerref) (`Character.CharacterMovement` (`self.CharacterRef`))))
    (else
      (bind _playerref_2 (message `/Game/_DEV/Interfaces/BPI_GetCombatCharacter.GetPlayerRef` (`self.CharacterRef`)))
      (`CombatProjectCharacter.ReleaseEnemy` _playerref_2)
      (set `self.bIsDraggingEnemy` false))))

(event `EnhancedInput|/Game/_DEV/Input/Actions/IA_Interact`
  (params (ActionValue :type Boolean) (ElapsedSeconds :type "Float (double-precision)") (TriggeredSeconds :type "Float (double-precision)") (InputAction :type "InputAction Object Reference" :default "/Game/_DEV/Input/Actions/IA_Interact.IA_Interact"))
  ;[0.7999 0.8475 1] InteractionWheelOpenClose
  (:`Started`
    (`KismetSystemLibrary.Delay` 0.01)
    (if (`self.bIsRadialWheelInteraction?`)
      (set `self.Is Wheel Open` (`self.Is Wheel Open`))
      (`/Game/Procedural_Radial_Wheel_Menu/Blueprints/Radial_Wheel_AC.Show Radial Wheel` (`self.Interactions Radial Wheel`))
      (`Controller.SetIgnoreMoveInput` (`Pawn.GetLocalViewingPlayerController` (`self.CharacterRef`)) true)
      (bind _interactions (message `/Game/_DEV/Interfaces/BPI_InteractionRadialWheel.GetInteractionOptions` (`self.F_GetActiveInteractable`)))
      (`self.AddOptionsToInteractionWheel` _interactions)))
  (:`Canceled`
    (if (`self.bIsRadialWheelInteraction?`) :!label _label
      (if (`self.Is Wheel Open`)
        (`/Game/Procedural_Radial_Wheel_Menu/Blueprints/Radial_Wheel_AC.Hide Radial Wheel` (`self.Interactions Radial Wheel`))
        (`Controller.SetIgnoreMoveInput` (`Pawn.GetLocalViewingPlayerController` (`self.CharacterRef`)) false)
        (`KismetSystemLibrary.Delay` 0.2)
        (`self.ClearInteractionWheel`))))
  (:`Completed`
    (goto _label)))

(event `RefreshInteractionWidget`
  ;[0.7999 0.8475 1] Refresh Interaction Widget
  (bind _interactionwidget (`self.F_RenderInteractionWidget`))
  (`self.F_InteractionWidgetSetup` (`self.F_GetActiveInteractable`) _interactionwidget))

(event `HandleBeginOverlap`
  (params (OverlappedComponent :type "PrimitiveComponent Object Reference") (OtherActor :type "Actor Object Reference") (OtherComp :type "PrimitiveComponent Object Reference") (OtherBodyIndex :type Integer) (bFromSweep :type Boolean) (SweepResult :type "HitResult Structure (by ref)"))
  ;[0.7999 0.8475 1] Begin Overlap
  (if (`KismetSystemLibrary.DoesImplementInterface` OtherActor "/Game/_DEV/Interfaces/BPI_Interactable.BPI_Interactable_C")
    (`KismetArrayLibrary.Array_AddUnique` (`self.InteractablesInRange`) OtherActor)
    (bind _interactionwidget (`self.F_RenderInteractionWidget`))
    (`self.F_InteractionWidgetSetup` (`self.F_GetActiveInteractable`) _interactionwidget)))

(event `AddOptionsToInteractionWheel`
  (params (InteractionName :type "Array of Name"))
  ;[0.7999 0.8475 1] RadialWheelAddSlots
  (for _array_element InteractionName
    (`/Game/Procedural_Radial_Wheel_Menu/Blueprints/Radial_Wheel_AC.Insert Slot` (`self.Interactions Radial Wheel`) 0 (make `/Game/Procedural_Radial_Wheel_Menu/Blueprints/Structs/Radial_Wheel_Slot_Struct` "/Game/Procedural_Radial_Wheel_Menu/Styles/Default/Radial_Wheel_Default_Style_DA.Radial_Wheel_Default_Style_DA" "/Game/Procedural_Radial_Wheel_Menu/Styles/Default/Radial_Wheel_Default_Active_Style_DA.Radial_Wheel_Default_Active_Style_DA" 1.0 false true (make `/Game/Procedural_Radial_Wheel_Menu/Blueprints/Structs/Radial_Wheel_Item_Struct` _array_element null (0.0 0.0) (struct :`Translation` (0.0 0.0) :`Scale` (1.0 1.0) :`Shear` (0.0 0.0)) (`KismetTextLibrary.Conv_NameToText` _array_element) (make `WidgetTransform` (0.0 0.0)))))))

(event `ClearInteractionWheel`
  (bind _interactions_radial_wheel (`self.Interactions Radial Wheel`))
  ;[0.7999 0.8475 1] RadialWheelAddSlots
  (`/Game/Procedural_Radial_Wheel_Menu/Blueprints/Radial_Wheel_AC.Clear Active Slots` _interactions_radial_wheel)
  (`/Game/Procedural_Radial_Wheel_Menu/Blueprints/Radial_Wheel_AC.Clear Active Slots` _interactions_radial_wheel))

(event `Interact_Disguise`
  (bind _activeinteractable (`self.F_GetActiveInteractable`))
  (bind (_returnvalue_x _returnvalue_y) (`KismetMathLibrary.BreakVector` (`Actor.K2_GetActorLocation` (`self.CharacterRef`))))
  ;[0.7999 0.8475 1] Disguise Body and Luggage
  (`/Engine/EditorBlueprintResources/StandardMacros.IsValid` _activeinteractable
    (:`Is Valid`
      (if (`KismetSystemLibrary.DoesImplementInterface` _activeinteractable "/Game/_DEV/Blueprints/Enemy/AI/BPI_EnemyAI.BPI_EnemyAI_C")
        (bind _enemyref (message `/Game/_DEV/Blueprints/Enemy/AI/BPI_EnemyAI.GetEnemyRef` (`self.F_GetActiveInteractable`)))
        (if (and (`/Game/_DEV/DamageSystem/BPC_DamageSystem.IsDead` (`/Game/_DEV/Blueprints/Enemy/BP_Enemy.BPC_DamageSystem` _enemyref)) (not (`/Game/_DEV/Blueprints/Enemy/BP_Enemy.bIsDisguised?` _enemyref)))
          (set `self.InBetweenCharacterClothes` (`SkeletalMeshComponent.SkeletalMeshAsset` (`Character.Mesh` (`self.CharacterRef`))))
          (`|PlayMontage` (`Character.Mesh` (`self.CharacterRef`)) "/Game/Loot_Anim_Set/Animations/Loot_Corpse/Loot_Corpse_GrabItem_Montage.Loot_Corpse_GrabItem_Montage"
            (:`OnNotifyBegin`
              (`SkeletalMeshComponent.SetSkeletalMeshAsset` (`Character.Mesh` (`self.CharacterRef`)) (`SkeletalMeshComponent.SkeletalMeshAsset` (`Character.Mesh` _enemyref)))
              (set `/Game/_DEV/Blueprints/Enemy/BP_Enemy.bIsDisguised?` true _enemyref)
              (`|SpawnActorFromClass` "/Game/_DEV/Blueprints/Interactables/BP_Backpack.BP_Backpack_C" (`KismetMathLibrary.MakeTransform` (`KismetMathLibrary.MakeVector` (+ _returnvalue_x 70.0) (+ _returnvalue_y 70.0))) "AdjustIfPossibleButAlwaysSpawn" "MultiplyWithRoot" null true (`self.InBetweenCharacterClothes`) null)
              (`SkeletalMeshComponent.SetSkeletalMeshAsset` (`Character.Mesh` _enemyref) "/Game/TSam_Agent/Character/Meshs/TSam_Agent/NagedAgent.NagedAgent")
              (`|PlayMontage` (`Character.Mesh` (`self.CharacterRef`)) "/Game/TryingOnClothesAnim/Animations/UE4/Male/A_M_Cloth_Torso_PutOn_Montage.A_M_Cloth_Torso_PutOn_Montage"
                (:`then`
                  (set `/Game/_DEV/Blueprints/Enemy/BP_Enemy.bIsNaked` true _enemyref)
                  (`self.RefreshInteractionWidget`))))))
        (elif (`KismetSystemLibrary.DoesImplementInterface` _activeinteractable "/Game/_DEV/Interfaces/BPI_GetBackpack.BPI_GetBackpack_C")
          (bind _backpackref (message `/Game/_DEV/Interfaces/BPI_GetBackpack.GetBackPackRef` (`self.F_GetActiveInteractable`)))
          (set `self.InBetweenCharacterClothes` (`SkeletalMeshComponent.SkeletalMeshAsset` (`Character.Mesh` (`self.CharacterRef`))))
          (`|PlayMontage` (`Character.Mesh` (`self.CharacterRef`)) "/Game/Loot_Anim_Set/Animations/Loot_Corpse/Loot_Corpse_GrabItem_Montage.Loot_Corpse_GrabItem_Montage"
            (:`OnNotifyBegin`
              (`SkeletalMeshComponent.SetSkeletalMeshAsset` (`Character.Mesh` (`self.CharacterRef`)) (`/Game/_DEV/Blueprints/Interactables/BP_Backpack.CurrentMesh` _backpackref))
              (set `/Game/_DEV/Blueprints/Interactables/BP_Backpack.CurrentMesh` (`self.InBetweenCharacterClothes`) _backpackref)
              (`/Game/_DEV/Blueprints/Interactables/BP_Backpack.UpdateBackpackContents_Clothes` _backpackref))))))))

(event `HandleEndOverlap`
  (params (OverlappedComponent :type "PrimitiveComponent Object Reference") (OtherActor :type "Actor Object Reference") (OtherComp :type "PrimitiveComponent Object Reference") (OtherBodyIndex :type Integer))
  ;[0.7999 0.8475 1] End Overlap
  (if (`KismetSystemLibrary.DoesImplementInterface` OtherActor "/Game/_DEV/Interfaces/BPI_Interactable.BPI_Interactable_C")
    (`KismetArrayLibrary.Array_RemoveItem` (`self.InteractablesInRange`) OtherActor)
    (`self.F_RenderInteractionWidget`)))

(event `InteractionWheelSlotChanged`
  (params (`Active Slot` :type "/Game/Procedural_Radial_Wheel_Menu/Blueprints/Structs/Radial_Wheel_Slot_Struct Structure"))
  ;[0.7999 0.8475 1] InteractionWheel
  (switch `name` (`KismetStringLibrary.Conv_StringToName` (`KismetStringLibrary.ToLower` (`KismetStringLibrary.Conv_NameToString` (`.Name_2_3A23B14B406942166AEFDE89E6E2E472` (break `/Game/Procedural_Radial_Wheel_Menu/Blueprints/Structs/Radial_Wheel_Item_Struct` (`.Item_12_0031A7584011B44C09CB79B714571AE8` (break `/Game/Procedural_Radial_Wheel_Menu/Blueprints/Structs/Radial_Wheel_Slot_Struct` `Active Slot`)))))))
    (:`loot`
      (`self.LootBody`))
    (:`drag`
      (`self.DragBody`))
    (:`disguise`
      (`self.Interact_Disguise`))))

(event `LootBody`
  ;[0.7999 0.8475 1] Loot Body
  (bind _enemyref (message `/Game/_DEV/Blueprints/Enemy/AI/BPI_EnemyAI.GetEnemyRef` (`self.F_GetActiveInteractable`)))
  (if (`/Game/_DEV/Blueprints/Enemy/BP_Enemy.bIsLooted` _enemyref)
    (`/Game/_DEV/UI/StealthGameUI/WBP_InGameStealth.SetInformationText` (`/Game/_DEV/Blueprints/BP_CombatCharacter.WBP Stealth Game UI` (`self.Player Ref`)) (`|FormatText` "Already Looted!"))
    (else
      (`|PlayMontage` (`Character.Mesh` (`self.CharacterRef`)) "/Game/Loot_Anim_Set/Animations/Loot_Corpse/Loot_Corpse_GrabItem_Montage.Loot_Corpse_GrabItem_Montage"
        (:`OnNotifyBegin`
          (set `/Game/_DEV/Blueprints/Enemy/BP_Enemy.bIsLooted` true _enemyref)
          (`/Game/_DEV/UI/StealthGameUI/WBP_InGameStealth.SetInformationText` (`/Game/_DEV/Blueprints/BP_CombatCharacter.WBP Stealth Game UI` (`self.Player Ref`)) (`|FormatText` "Nothing Found!")))))))

(event `EnhancedInput|/Game/_DEV/Input/Actions/IA_Interact`
  (params (ActionValue :type Boolean) (ElapsedSeconds :type "Float (double-precision)") (TriggeredSeconds :type "Float (double-precision)") (InputAction :type "InputAction Object Reference" :default "/Game/_DEV/Input/Actions/IA_Interact.IA_Interact"))
  (bind _output (`|GetArrayItem` (`self.InteractablesInRange`)))
  ;[0.7999 0.8475 1] Interact
  (:`Started`
    (if (`KismetArrayLibrary.Array_IsNotEmpty` (`self.InteractablesInRange`))
      (bind _itemref (message `/Game/_DEV/Interfaces/BPI_Interactable.GetItemRef` _output))
      (`/Engine/EditorBlueprintResources/StandardMacros.IsValid` _itemref
        (:`Is Valid`
          (if (not (`/Game/_DEV/Blueprints/Interactables/BP_InteractItemBase.bIsInteracting` _itemref))
            (set `/Game/_DEV/Blueprints/Interactables/BP_InteractItemBase.bIsInteracting` true _itemref)
            (bind _interactiontype (message `/Game/_DEV/Interfaces/BPI_Interactable.GetTypeOfInteraction` _itemref))
            (switch `/Game/_DEV/Enums/E_TypesOfInteraction` _interactiontype
              (:`NewEnumerator0`
                (bind _interactanimmontage (`/Game/_DEV/Blueprints/Interactables/BP_InteractItemBase.InteractAnimMontage` _itemref)
                  (:`then`
                    (`|PlayMontage` (`Character.Mesh` (`self.CharacterRef`)) _interactanimmontage
                      (:`OnNotifyBegin`
                        _)))
                  (:`else`
                    _)))
              (:`NewEnumerator7`
                _)
              (:`NewEnumerator8`
                (`self.F_CalculateItemDistanceAndSetAnimation` _itemref)
                (`|PlayMontage` (`Character.Mesh` (`self.CharacterRef`)) (`self.PickupAnimMontageToPlayBasedOnDistance`) 1.4
                  (:`OnNotifyBegin`
                    _)))
              (:`NewEnumerator9`
                _))
            (message `/Game/_DEV/Interfaces/BPI_Interactable.Interact` (`self.F_GetActiveInteractable`) (`self.GetOwner`))))
        (:`Is Not Valid`
          (bind _enemyref (message `/Game/_DEV/Blueprints/Enemy/AI/BPI_EnemyAI.GetEnemyRef` _output))
          (bind _interactiontype_2 (message `/Game/_DEV/Interfaces/BPI_Interactable.GetTypeOfInteraction` _enemyref))
          (switch `/Game/_DEV/Enums/E_TypesOfInteraction` _interactiontype_2
            (:`NewEnumerator3`
              (set `self.bIsRadialWheelInteraction?` true))))))))

(fn `F_CalculateItemDistanceAndSetAnimation`
  (params (Interactable :type "Actor Object Reference"))
  (locals (DistanceOfItemToGround :type "Float (double-precision)") (AnimationValue :type Integer))
  (bind _returnvalue (`Actor.K2_GetActorLocation` Interactable))
  (bind _outhit (`KismetSystemLibrary.LineTraceSingle` _returnvalue (- _returnvalue (0.0 0.0 1000.0)) "TraceTypeQuery1"))
  (set `local.DistanceOfItemToGround` (- (.z _returnvalue) (.z (`.ImpactPoint` (`GameplayStatics.BreakHitResult` _outhit)))))
  (if (<= (`local.DistanceOfItemToGround`) 0.0)
    (set `self.PickupAnimMontageToPlayBasedOnDistance` "/Game/ItemPickupSet/Animations/Mannequin_UE4/fromIdle/A_ItemPickup_fromIdle_RH_0cm_Montage.A_ItemPickup_fromIdle_RH_0cm_Montage")
    (elif (<= (`local.DistanceOfItemToGround`) 25.0)
      (set `self.PickupAnimMontageToPlayBasedOnDistance` "/Game/ItemPickupSet/Animations/Mannequin_UE4/fromIdle/A_ItemPickup_fromIdle_RH_25cm_Montage.A_ItemPickup_fromIdle_RH_25cm_Montage")
      (elif (<= (`local.DistanceOfItemToGround`) 50.0)
        (set `self.PickupAnimMontageToPlayBasedOnDistance` "/Game/ItemPickupSet/Animations/Mannequin_UE4/fromIdle/A_ItemPickup_fromIdle_RH_50cm_Montage.A_ItemPickup_fromIdle_RH_50cm_Montage")
        (elif (<= (`local.DistanceOfItemToGround`) 75.0)
          (set `self.PickupAnimMontageToPlayBasedOnDistance` "/Game/ItemPickupSet/Animations/Mannequin_UE4/fromIdle/A_ItemPickup_fromIdle_RH_75cm_Montage.A_ItemPickup_fromIdle_RH_75cm_Montage")
          (elif (<= (`local.DistanceOfItemToGround`) 100.0)
            (set `self.PickupAnimMontageToPlayBasedOnDistance` "/Game/ItemPickupSet/Animations/Mannequin_UE4/fromIdle/A_ItemPickup_fromIdle_RH_100cm_Montage.A_ItemPickup_fromIdle_RH_100cm_Montage")
            (elif (<= (`local.DistanceOfItemToGround`) 125.0)
              (set `self.PickupAnimMontageToPlayBasedOnDistance` "/Game/ItemPickupSet/Animations/Mannequin_UE4/fromIdle/A_ItemPickup_fromIdle_RH_125cm_Montage.A_ItemPickup_fromIdle_RH_125cm_Montage")
              (elif (<= (`local.DistanceOfItemToGround`) 150.0)
                (set `self.PickupAnimMontageToPlayBasedOnDistance` "/Game/ItemPickupSet/Animations/Mannequin_UE4/fromIdle/A_ItemPickup_fromIdle_RH_150cm_Montage.A_ItemPickup_fromIdle_RH_150cm_Montage")
                (elif (<= (`local.DistanceOfItemToGround`) 175.0)
                  (set `self.PickupAnimMontageToPlayBasedOnDistance` "/Game/ItemPickupSet/Animations/Mannequin_UE4/fromIdle/A_ItemPickup_fromIdle_RH_175cm_Montage.A_ItemPickup_fromIdle_RH_175cm_Montage")
                  (elif (<= (`local.DistanceOfItemToGround`) 200.0)
                    (set `self.PickupAnimMontageToPlayBasedOnDistance` "/Game/ItemPickupSet/Animations/Mannequin_UE4/fromIdle/A_ItemPickup_fromIdle_RH_200cm_Montage.A_ItemPickup_fromIdle_RH_200cm_Montage")))))))))))

(fn `F_GetActiveInteractable`
  (returns (ActiveInteractable :type "Actor Object Reference"))
  (bind _interactablesinrange (`self.InteractablesInRange`))
  (return (`|GetArrayItem` _interactablesinrange (`KismetArrayLibrary.Array_LastIndex` _interactablesinrange))))

(fn `F_InteractionWidgetSetup`
  (params (Target :type "Object Object Reference") (Widget :type "/Game/_DEV/Blueprints/Interactables/NEW/WBP_Interaction Object Reference"))
  (bind (_interactiontext _getkeyimage) (message `/Game/_DEV/Interfaces/BPI_Interactable.GetInteractionText` Target))
  (set `/Game/_DEV/Blueprints/Interactables/NEW/WBP_Interaction.InteractionPrompt` _interactiontext Widget)
  (set `/Game/_DEV/Blueprints/Interactables/NEW/WBP_Interaction.InteractionImage` _getkeyimage Widget))

(fn `F_RenderInteractionWidget`
  (returns (InteractionWidget :type "/Game/_DEV/Blueprints/Interactables/NEW/WBP_Interaction Object Reference"))
  (bind _interactionwidgetcomponent (`self.InteractionWidgetComponent`))
  (if (`KismetArrayLibrary.Array_IsNotEmpty` (`self.InteractablesInRange`))
    (bind _returnvalue (`|CreateWidget` "/Game/_DEV/Blueprints/Interactables/NEW/WBP_Interaction.WBP_Interaction_C"))
    (`WidgetComponent.SetWidget` _interactionwidgetcomponent _returnvalue)
    (`SceneComponent.K2_SetWorldLocation` _interactionwidgetcomponent (`Actor.K2_GetActorLocation` (`self.F_GetActiveInteractable`)) false false)
    (return _returnvalue)
    (else
      (`WidgetComponent.SetWidget` (`self.InteractionWidgetComponent`) null))))