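; BP_BlendInteractable is an interactable that lets the player toggle a "blending in" animation on and off.
; Interact plays BlendingAnimationToPlay on the player's mesh and replays it on completion, or stops the montage if it is already playing.
; Both paths update the playing flag, refresh the player's interaction widget and clear IsInteracting.
; The prompt text switches between start and stop based on that flag.
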(event `/Game/_DEV/Interfaces/BPI_Interactable.Interact`
  (params (InterActor :type "Actor Object Reference"))
  (if (not (`self.Is Playing Blending Animation`))
    (bind _playerref (message `/Game/_DEV/Interfaces/BPI_GetCombatCharacter.GetPlayerRef` InterActor :!label _label))
    (`|PlayMontage` (`Character.Mesh` _playerref) (`self.BlendingAnimationToPlay`)
      (:`then`
        (set `self.Is Playing Blending Animation` true)
        (`/Game/_DEV/Blueprints/ActorComponents/PlayerInteractionsComponent.RefreshInteractionWidget` (`/Game/_DEV/Blueprints/BP_CombatCharacter.PlayerInteractionComponent` _playerref)))
      (:`OnCompleted`
        (goto _label)))
    (else
      (bind _playerref_2 (message `/Game/_DEV/Interfaces/BPI_GetCombatCharacter.GetPlayerRef` InterActor))
      (`/Game/_DEV/Blueprints/BP_CombatCharacter.StopMontageFromPlaying` _playerref_2)
      (set `self.Is Playing Blending Animation` false)
      (`/Game/_DEV/Blueprints/ActorComponents/PlayerInteractionsComponent.RefreshInteractionWidget` (`/Game/_DEV/Blueprints/BP_CombatCharacter.PlayerInteractionComponent` _playerref_2))))
  (set `self.bIsInteracting` false))

(fn `GetInteractionText`
  (returns (InteractionText :type Text) (GetKeyImage :type "Texture Object Reference"))
  (if (`self.Is Playing Blending Animation`)
    (return "Stop blending in" "/Game/_DEV/Misc/KeyboardButtons/keyboard_e.keyboard_e")
    (else
      (return "Start blending in" "/Game/_DEV/Misc/KeyboardButtons/keyboard_e.keyboard_e"))))

(fn `GetItemRef`
  (returns (ItemRef :type "/Game/_DEV/Blueprints/Interactables/BP_InteractItemBase Object Reference"))
  (return self))

(fn `GetTypeOfInteraction`
  (returns (InteractionType :type "/Game/_DEV/Enums/E_TypesOfInteraction Enum"))
  (return "NewEnumerator9"))

(fn `UserConstructionScript`
  (`parent.UserConstructionScript`))