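; BP_DoorButton is an interactable button that opens and closes a referenced door.
; Interact plays or reverses a Timeline based on IsDoorOpened, and that flag flips when the Timeline finishes.
; The Timeline's ZRotation track, despite its name, slides the door mesh along relative X at a fixed Z.
; Interaction getters supply a self reference, an interaction type and the "Press Button" prompt.
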(event `/Game/_DEV/Interfaces/BPI_Interactable.Interact`
  (params (InterActor :type "Actor Object Reference"))
  (if (not (`self.bIsDoorOpened`))
    (bind (_direction _zrotation) (`Timeline|Timeline` :!label _label)
      (:`Update`
        (`SceneComponent.K2_SetRelativeLocation` (`/Game/_DEV/Blueprints/Interactables/BP_InteractItemBase.Mesh` (`self.RespectiveDoor`)) (`KismetMathLibrary.MakeVector` _zrotation 0.0 -100.0) false false))
      (:`Finished`
        (if (`self.bIsDoorOpened`)
          (set `self.bIsDoorOpened` false)
          (else
            (set `self.bIsDoorOpened` true)))
        (set `self.bIsInteracting` false)))
    (else
      (goto _label :!via `Reverse`))))

(fn `GetInteractionText`
  (returns (InteractionText :type Text))
  (return (`|FormatText` "Press Button")))

(fn `GetItemRef`
  (returns (ItemRef :type "/Game/_DEV/Blueprints/Interactables/BP_InteractItemBase Object Reference"))
  (return self))

(fn `GetTypeOfInteraction`
  (returns (InteractionType :type "/Game/_DEV/Enums/E_TypesOfInteraction Enum"))
  (return "NewEnumerator0"))

(fn `UserConstructionScript`
  (`parent.UserConstructionScript`))