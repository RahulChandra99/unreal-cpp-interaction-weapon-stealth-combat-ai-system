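; BP_Door is an interactable door whose status (unlocked, locked or button) sets its mesh, frame visibility and prompt text.
; Interact plays character montages: notifies open or close unlocked doors, while locked doors unlock if the player's CanUnlocked flag is set.
; A timeline drives the swing, using a dot product to choose direction from the interactor's side, and reverses to close.
; Button doors have a prompt but no Interact handling here.
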(event `self.ReceiveBeginPlay`
  (bind _mesh (`self.Mesh`))
  ;[0.7999 0.8475 1] Begin Play, Door Mesh Setup[
  (switch `/Game/_DEV/Enums/E_TypeOfDoor` (`self.DoorStatus`)
    (:`NewEnumerator0`
      (`StaticMeshComponent.SetStaticMesh` _mesh "/Game/DoorsPack/Meshes/SM_DoorDouble02_DoorL.SM_DoorDouble02_DoorL")
      (`SceneComponent.SetVisibility` (`self.Frame`) true false))
    (:`NewEnumerator1`
      (`StaticMeshComponent.SetStaticMesh` _mesh "/Game/ThirdPersonDoors/Meshes/SM_Door_Knob.SM_Door_Knob")
      (`SceneComponent.SetVisibility` (`self.Frame`) false false))
    (:`NewEnumerator2`
      (`StaticMeshComponent.SetStaticMesh` _mesh "/Game/DoorsPack/Meshes/SM_DoorDouble01_DoorL.SM_DoorDouble01_DoorL")
      (`SceneComponent.SetVisibility` (`self.Frame`) false false))))

(event `OpenDoor`
  ;[0.7999 0.8475 1] Open door Close Animation
  (`GameplayStatics.PlaySoundAtLocation` "/Game/BlockingStarterPack/Sounds/SimpleDoor_StartOpening01.SimpleDoor_StartOpening01" (`self.K2_GetActorLocation`) (struct) 1.0 1.0 0.0 null null null null)
  (set `self.Direction` (> (`KismetMathLibrary.Dot_VectorVector` (`self.GetActorRightVector`) (`KismetMathLibrary.Normal` (- (`self.K2_GetActorLocation` (`self.InterActor`)) (`self.K2_GetActorLocation`)))) 0.0))
  (bind (_direction _zrotation) (`Timeline|OpenDoorTimeline` :!label _label)
    (:`Update`
      (`SceneComponent.K2_SetRelativeRotation` (`self.Mesh`) (`KismetMathLibrary.MakeRotator` 0.0 0.0 (* _zrotation (`KismetMathLibrary.SelectFloat` -1.0 1.0 (`self.Direction`)))) false false))
    (:`Finished`
      (if (`self.bIsDoorOpen`)
        (set `self.bIsDoorOpen` false)
        (`GameplayStatics.PlaySoundAtLocation` "/Game/BlockingStarterPack/Sounds/SimpleDoor_Closing01.SimpleDoor_Closing01" (`self.K2_GetActorLocation`) (struct) 1.0 1.0 0.0 null null null null)
        (else
          (set `self.bIsDoorOpen` true))))))

(event `CloseDoor`
  ;[0.7999 0.8475 1] Open door Close Animation
  (goto _label :!via `ReverseFromEnd`))

(event `/Game/_DEV/Interfaces/BPI_Interactable.Interact`
  (params (InterActor :type "Actor Object Reference"))
  (bind _output_get (set `self.InterActor` InterActor))
  (bind _ascharacter (cast `Character` _output_get))
  (switch `/Game/_DEV/Enums/E_TypeOfDoor` (`self.DoorStatus`)
    (:`NewEnumerator0`
      (if (`self.bIsDoorOpen`)
        (bind _playerref (message `/Game/_DEV/Interfaces/BPI_GetCombatCharacter.GetPlayerRef` (`self.InterActor`)))
        (bind _mesh (`Character.Mesh` _ascharacter))
        (`|PlayMontage` _mesh "/Game/ThirdPersonDoors/Animations/RootMotion/RM_Front_Lever_Close_Montage.RM_Front_Lever_Close_Montage"
          (:`OnNotifyBegin`
            (`self.CloseDoor`)
            (`/Game/_DEV/Blueprints/ActorComponents/PlayerInteractionsComponent.RefreshInteractionWidget` (`/Game/_DEV/Blueprints/BP_CombatCharacter.PlayerInteractionComponent` _playerref))
            (set `self.bIsInteracting` false)))
        (else
          (bind _playerref_2 (message `/Game/_DEV/Interfaces/BPI_GetCombatCharacter.GetPlayerRef` (`self.InterActor`)))
          (`|PlayMontage` _mesh "/Game/ThirdPersonDoors/Animations/RootMotion/RM_Front_Lever_Open_Montage.RM_Front_Lever_Open_Montage"
            (:`OnNotifyBegin`
              (`self.OpenDoor`)
              (`/Game/_DEV/Blueprints/ActorComponents/PlayerInteractionsComponent.RefreshInteractionWidget` (`/Game/_DEV/Blueprints/BP_CombatCharacter.PlayerInteractionComponent` _playerref_2))
              (set `self.bIsInteracting` false))))))
    (:`NewEnumerator1`
      (bind _playerref_3 (message `/Game/_DEV/Interfaces/BPI_GetCombatCharacter.GetPlayerRef` (`self.InterActor`)))
      (if (`/Game/_DEV/Blueprints/BP_CombatCharacter.bCanUnlocked` _playerref_3)
        (`|PlayMontage` _mesh "/Game/Loot_Anim_Set/Animations/Loot_Dresser/Loot_Dresser_GrabItem_Montage.Loot_Dresser_GrabItem_Montage"
          (:`OnCompleted`
            (set `self.DoorStatus` "NewEnumerator0")
            (`/Game/_DEV/Blueprints/ActorComponents/PlayerInteractionsComponent.RefreshInteractionWidget` (`/Game/_DEV/Blueprints/BP_CombatCharacter.PlayerInteractionComponent` _playerref_3))
            (set `self.bIsInteracting` false)))
        (else
          (`|PlayMontage` _mesh "/Game/ThirdPersonDoors/Animations/RootMotion/RM_Front_Knob_Locked_Montage.RM_Front_Knob_Locked_Montage"
            (:`OnCompleted`
              (`/Game/_DEV/Blueprints/ActorComponents/PlayerInteractionsComponent.RefreshInteractionWidget` (`/Game/_DEV/Blueprints/BP_CombatCharacter.PlayerInteractionComponent` _playerref_3))
              (set `self.bIsInteracting` false))))))))

(fn `GetInteractionText`
  (returns (InteractionText :type Text) (GetKeyImage :type "Texture Object Reference"))
  (switch `/Game/_DEV/Enums/E_TypeOfDoor` (`self.DoorStatus`)
    (:`NewEnumerator0`
      (if (`self.bIsDoorOpen`)
        (return "Close Door" "/Game/_DEV/Misc/KeyboardButtons/keyboard_e.keyboard_e")
        (else
          (return "Open Door" "/Game/_DEV/Misc/KeyboardButtons/keyboard_e.keyboard_e"))))
    (:`NewEnumerator1`
      (return "Locked, requires key" "/Game/_DEV/Misc/KeyboardButtons/keyboard_e.keyboard_e"))
    (:`NewEnumerator2`
      (return "Use Button" "/Game/_DEV/Misc/KeyboardButtons/keyboard_e.keyboard_e"))))

(fn `GetItemRef`
  (returns (ItemRef :type "/Game/_DEV/Blueprints/Interactables/BP_InteractItemBase Object Reference"))
  (return self))

(fn `UserConstructionScript`)