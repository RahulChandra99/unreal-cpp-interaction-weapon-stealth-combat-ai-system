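; BP_Backpack is an interactable backpack that lets the player disguise into the clothes it holds.
; On BeginPlay and content updates, it derives its information text from the current mesh if it has clothes, feeding the "Disguise into" prompt with an E-key image.
; Interacting fetches the player reference and delegates the disguise to its PlayerInteractionComponent.
; Getter functions expose the backpack reference and interaction type.
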(event `self.ReceiveBeginPlay`
  (`self.UpdateBackpackContents_Clothes`))

(event `UpdateBackpackContents_Clothes`
  (if (`self.bHasClothes?`)
    (bind _output_get (set `self.CurrentMesh` (`self.CurrentMesh`)))
    (set `self.Information Text` (`KismetTextLibrary.Conv_ObjectToText` _output_get))))

(event `/Game/_DEV/Interfaces/BPI_Interactable.Interact`
  (params (InterActor :type "Actor Object Reference"))
  (bind _playerref (message `/Game/_DEV/Interfaces/BPI_GetCombatCharacter.GetPlayerRef` InterActor))
  (`/Game/_DEV/Blueprints/ActorComponents/PlayerInteractionsComponent.Interact_Disguise` (`/Game/_DEV/Blueprints/BP_CombatCharacter.PlayerInteractionComponent` _playerref))
  (set `self.bIsInteracting` false))

(fn `GetBackPackRef`
  (returns (BackpackRef :type "/Game/_DEV/Blueprints/Interactables/BP_Backpack Object Reference"))
  (return self))

(fn `GetInteractionText`
  (returns (InteractionText :type Text) (GetKeyImage :type "Texture Object Reference"))
  (return (`|FormatText` "Disguise into {clothes} " (`self.Information Text`)) "/Game/_DEV/Misc/KeyboardButtons/keyboard_e.keyboard_e"))

(fn `GetItemRef`
  (returns (ItemRef :type "/Game/_DEV/Blueprints/Interactables/BP_InteractItemBase Object Reference"))
  (return self))

(fn `GetTypeOfInteraction`
  (returns (InteractionType :type "/Game/_DEV/Enums/E_TypesOfInteraction Enum"))
  (return "NewEnumerator7"))

(fn `UserConstructionScript`)