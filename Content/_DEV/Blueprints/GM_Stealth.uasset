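; GM_Stealth is the game mode for stealth play, handling the player's start location and stealth HUD.
; PostLogin restarts player 0 at the "StealthLocation" player start, then runs the same setup as BeginPlay.
; That setup creates WBP_InGameStealth if needed, adds it to the viewport and sets TypeOfGame on the player's BP_CombatCharacter.
; GetStealthGM returns the game mode itself.
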(event `self.ReceiveBeginPlay`
  (bind _wbp_stealthgameui (`self.WBP StealthGameUI` :!label _label)
    (:`then`
      _)
    (:`else`
      (bind _returnvalue (`|CreateWidget` "/Game/_DEV/UI/StealthGameUI/WBP_InGameStealth.WBP_InGameStealth_C"))
      (bind _output_get (set `self.WBP StealthGameUI` _returnvalue))))
  (`UserWidget.AddToViewport` _output_get 0)
  (`UserWidget.AddToViewport` _wbp_stealthgameui 0)
  (bind _asbp_combat_character (cast `/Game/_DEV/Blueprints/BP_CombatCharacter` (`GameplayStatics.GetPlayerPawn` 0)))
  (set `/Game/_DEV/Blueprints/BP_CombatCharacter.TypeOfGame` "NewEnumerator1" _asbp_combat_character))

(event `self.K2_PostLogin`
  (params (NewPlayer :type "PlayerController Object Reference"))
  (`self.RestartPlayerAtPlayerStart` (`GameplayStatics.GetPlayerController` 0) (`self.K2_FindPlayerStart` (`GameplayStatics.GetPlayerController` 0) "StealthLocation"))
  (goto _label))

(fn `GetStealthGM`
  (returns (StealthGameMode :type "/Game/_DEV/Blueprints/GM_Stealth Object Reference"))
  (return self))

(fn `UserConstructionScript`)