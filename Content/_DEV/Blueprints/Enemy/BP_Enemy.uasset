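; BP_Enemy is the enemy character that patrols, fights with a katana and can be assassinated, looted, dragged or disguised from.
; BPCDamageSystem handles health, with its death, block and damage-response events bound in the construction script.
; Stealth types get a random outfit and optional rifle at BeginPlay.
; Takedowns play victim montages from DT_WeaponType by player weapon and direction, then ragdoll; interaction prompts switch on death.
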(event `self.SenseEnemyVisual`
  (params (bEnable :type Boolean))
  ;[0.7999 0.8475 1] Sense Ability
  (`SceneComponent.SetVisibility` (`self.OverheadWidget`) bEnable false))

(event `LootingBody`)

(event `InitializeEnemy`
  (switch `/Game/_DEV/Enums/E_TypeOfEnemy` (`self.TypeOfEnemy`)))

(event `self.ReceiveBeginPlay`
  (bind _stealthguardhair (`self.StealthGuardHair`))
  ;[0.7999 0.8475 1] Begin Play
  (`PlayerController.SetViewTargetWithBlend` (`GameplayStatics.GetPlayerController` 0) (`self.New View Target`) 0.0 "VTBlend_Linear" 0.0 false)
  (switch `/Game/_DEV/Enums/E_TypeOfEnemy` (`self.EnemyType`)
    (:`NewEnumerator3`
      (if (`self.bIsHoldingRifle`)
        (bind _returnvalue (`|SpawnActorFromClass` "/Game/_DEV/Blueprints/Weapon/Stealth/BP_Rifle.BP_Rifle_C" (`KismetMathLibrary.MakeTransform` (0.0 0.0 0.0)) "AdjustIfPossibleButAlwaysSpawn" "MultiplyWithRoot" null null))
        ;;[0.01096 0.01161 0.0137] SetStealthMesh
        (`self.K2_AttachToComponent` _returnvalue (`self.Mesh`) "RifleEquipSocket" "SnapToTarget" "SnapToTarget" "SnapToTarget" true))
      (`SceneComponent.SetVisibility` _stealthguardhair true false)
      (`SceneComponent.K2_AttachToComponent` _stealthguardhair (`self.Mesh`) "HairSocket" "SnapToTarget" "SnapToTarget" "SnapToTarget" true)
      (switch `int` (`KismetMathLibrary.RandomInteger` 4)
        (:`0`
          (`SkeletalMeshComponent.SetSkeletalMeshAsset` (`self.Mesh`) "/Game/TSam_Agent/Character/Meshs/TSam_Agent/BlackSweater.BlackSweater"))
        (:`1`
          (`SkeletalMeshComponent.SetSkeletalMeshAsset` (`self.Mesh`) "/Game/TSam_Agent/Character/Meshs/TSam_Agent/BlueSweater.BlueSweater"))
        (:`2`
          (`SkeletalMeshComponent.SetSkeletalMeshAsset` (`self.Mesh`) "/Game/TSam_Agent/Character/Meshs/TSam_Agent/GreenSuit.GreenSuit"))
        (:`3`
          (`SkeletalMeshComponent.SetSkeletalMeshAsset` (`self.Mesh`) "/Game/TSam_Agent/Character/Meshs/TSam_Agent/GreenSweater.GreenSweater"))))))

(event `EnemyInterface.OnLockonSelect`
  ;[0.7999 0.8475 1] Target LockOn
  (`SceneComponent.SetVisibility` (`self.LockOnWidget`) true false))

(event `EnemyInterface.OnLockonDeSelect`
  ;[0.7999 0.8475 1] Target LockOn
  (`SceneComponent.SetVisibility` (`self.LockOnWidget`) false false))

(event `self.OnStealthTakeDownVictim`
  ;[0.7999 0.8475 1] Stealth Takedown
  (`PrimitiveComponent.SetCollisionResponseToChannel` (`self.CapsuleComponent`) "ECC_Pawn" "ECR_Ignore")
  (bind _asbp_combat_character (cast `/Game/_DEV/Blueprints/BP_CombatCharacter` (`GameplayStatics.GetPlayerCharacter` 0)))
  (bind _output_get (set `self.CombatPlayerRef` _asbp_combat_character))
  (if (`/Game/_DEV/Blueprints/BP_CombatCharacter.IsTakedownFromBehind` _output_get)
    (bind _returnvalue (`|GetDataTableRow` "/Game/_DEV/DataTable/Weapon/DT_WeaponType.DT_WeaponType" (`/Game/_DEV/Blueprints/Weapon/BP_BaseWeapon.WeaponName` (`/Game/_DEV/Blueprints/BP_CombatCharacter.EquippedWeapon` (`self.CombatPlayerRef`))))
      (:`then`
        (`|PlayMontage` (`self.Mesh`) (`|GetArrayItem` (`.TakedownBehindVictimMontage_37_6B2155364EFEB97B9A3EB4B66AA49321` (break `/Game/_DEV/DataTable/Weapon/S_WeaponType` _returnvalue))))))
    (else
      (bind _returnvalue_2 (`|GetDataTableRow` "/Game/_DEV/DataTable/Weapon/DT_WeaponType.DT_WeaponType" (`/Game/_DEV/Blueprints/Weapon/BP_BaseWeapon.WeaponName` (`/Game/_DEV/Blueprints/BP_CombatCharacter.EquippedWeapon` (`self.CombatPlayerRef`))))
        (:`then`
          (`|PlayMontage` (`self.Mesh`) (`|GetArrayItem` (`.TakedownFrontVictimMontage_39_92D6B8D844B4F54298C4E2AABAB2042A` (break `/Game/_DEV/DataTable/Weapon/S_WeaponType` _returnvalue_2)))))))))

(event `self.OnStealthTakeDownVictim_End`
  ;[0.7999 0.8475 1] Stealth Takedown
  (`PrimitiveComponent.SetCollisionEnabled` (`self.Mesh`) "QueryAndPhysics")
  (`SkeletalMeshComponent.SetAllBodiesBelowSimulatePhysics` (`self.Mesh`) "pelvis" true true)
  (`PrimitiveComponent.SetCollisionEnabled` (`self.CapsuleComponent`) "NoCollision")
  (`PrimitiveComponent.SetEnableGravity` (`self.CapsuleComponent`) false)
  (set `/Game/_DEV/DamageSystem/BPC_DamageSystem.IsDead` true (`self.BPC_DamageSystem`)))

(event `self.RagdollDeath`
  ;[0.7999 0.8475 1] Damage System
  (set `/Game/_DEV/DamageSystem/BPC_DamageSystem.IsDead` true (`self.BPC_DamageSystem`)))

(event `Death`
  (bind _mesh (`self.Mesh`))
  ;[0.7999 0.8475 1] Damage System
  (`PrimitiveComponent.SetSimulatePhysics` _mesh true)
  (`PrimitiveComponent.SetCollisionEnabled` _mesh "QueryAndPhysics")
  (`PrimitiveComponent.SetCollisionEnabled` (`self.CapsuleComponent`) "NoCollision"))

(event `Blocked`
  (params (CanBeParried :type Boolean))
  ;[0.7999 0.8475 1] Damage System
  (`KismetSystemLibrary.PrintString` "Blocked"))

(event `DamageResponse`
  (params (DamageResponse :type "/Game/_DEV/DamageSystem/E_DamageResponses Enum" :default "NewEnumerator0"))
  ;[0.7999 0.8475 1] Damage System
  (switch `/Game/_DEV/DamageSystem/E_DamageResponses` DamageResponse
    (:`NewEnumerator1`
      (`|PlayMontage` (`self.Mesh`) "/Game/BMMCSystem/Animations/Combat/Other/A_DrawWeaponTemp_Montage.A_DrawWeaponTemp_Montage"))))

(event `MoveTo`
  (params (Location :type "Vector Structure") (Rotation :type "Rotator Structure"))
  (`|AIMoveTo` self Location null
    (:`OnSuccess`
      (`self.PlayAnimMontage` "/Game/TDA_PACK/Animations/InPlace/Axe/Behind_1/CharB_Axe_B1_Montage.CharB_Axe_B1_Montage")
      (`self.K2_SetActorRotation` Rotation))))

(event `AssignWeapon`
  (`|PlayMontage` (`self.Mesh`) "/Game/_DEV/Animations/AM_Unequip.AM_Unequip"
    (:`OnCompleted`
      (`self.OnWieldWeapon`))
    (:`OnNotifyBegin`
      (bind _returnvalue (`|SpawnActorFromClass` "/Game/_DEV/Blueprints/Weapon/Combat/BP_Katana.BP_Katana_C" (`self.GetTransform`) "Undefined" "MultiplyWithRoot" null null))
      (bind _output_get (set `self.Weapon` _returnvalue))
      (`self.K2_AttachToComponent` _output_get (`self.Mesh`) "KatanaEquipSocket" "SnapToTarget" "SnapToTarget" "SnapToTarget" true)
      (set `self.IsWieldingWeapon` true))))

(event `Attack`
  (`|PlayMontage` (`self.Mesh`) "/Game/BoStaff_AnimSet/Animation/attack_01_Montage.attack_01_Montage"
    (:`OnCompleted`
      _)
    (:`OnInterrupted`
      _))
  (`self.OnAttackEnd`))

(event `SheathSword`
  (bind _notifyname (`|PlayMontage` (`self.Mesh`) "/Game/_DEV/Animations/AM_Unequip.AM_Unequip")
    (:`OnCompleted`
      (`self.OnSheathWeapon`))
    (:`OnNotifyBegin`
      (switch `name` _notifyname
        (:`Drop`
          (`self.K2_DestroyActor` (`self.Weapon`))
          (set `self.IsWiedlingWeapon` false))))))

(fn `CheckStamina`
  (returns (IsStaminaLeft :type Boolean))
  (return false))

(fn `GetCurrentHealth`
  (returns (Health :type "Float (double-precision)"))
  (return (`/Game/_DEV/DamageSystem/BPC_DamageSystem.Health` (`self.BPC_DamageSystem`))))

(fn `GetCurrentStamina`
  (returns (Stamina :type "Float (double-precision)"))
  (return 0.0))

(fn `GetEnemyRef`
  (returns (EnemyRef :type "/Game/_DEV/Blueprints/Enemy/BP_Enemy Object Reference"))
  (return self))

(fn `GetInteractionOptions`
  (returns (Interactions :type "Array of Name"))
  (if (not (`self.bIsNaked`))
    (return (`|MakeArray` "Loot" "Drag" "Disguise" :!type "Name"))
    (else
      (return (`|MakeArray` "Loot" "Drag" :!type "Name")))))

(fn `GetInteractionText`
  (returns (InteractionText :type Text) (GetKeyImage :type "Texture Object Reference"))
  (if (not (`/Game/_DEV/DamageSystem/BPC_DamageSystem.IsDead` (`self.BPC_DamageSystem`)))
    (return "Assassinate" "/Game/_DEV/Misc/KeyboardButtons/keyboard_q.keyboard_q")
    (else
      (return "Interact" "/Game/_DEV/Misc/KeyboardButtons/keyboard_e.keyboard_e"))))

(fn `GetItemRef`
  (returns (ItemRef :type "/Game/_DEV/Blueprints/Interactables/BP_InteractItemBase Object Reference"))
  (return null))

(fn `GetMaterials`
  (returns (EnemyClothes :type "Array of MaterialInterface Object Reference"))
  (return (`MeshComponent.GetMaterials` (`self.Mesh`))))

(fn `GetMaxHealth`
  (returns (MaxHealth :type "Float (double-precision)"))
  (return (`/Game/_DEV/DamageSystem/BPC_DamageSystem.MaxHealth` (`self.BPC_DamageSystem`))))

(fn `GetMaxStamina`
  (returns (MaxStamina :type "Float (double-precision)"))
  (return 0.0))

(fn `GetPatrolRoute`
  (returns (PatrolRoute :type "/Game/_DEV/Blueprints/Enemy/AI/BP_PatrolRoute Object Reference"))
  (return (`self.PatrolRoute`)))

(fn `GetTypeOfInteraction`
  (returns (InteractionType :type "/Game/_DEV/Enums/E_TypesOfInteraction Enum"))
  (if (`/Game/_DEV/DamageSystem/BPC_DamageSystem.IsDead` (`self.BPC_DamageSystem`))
    (return "NewEnumerator3")
    (else
      (return "NewEnumerator5"))))

(fn `Heal`
  (params (Amount :type "Float (double-precision)"))
  (returns (NewHealth :type "Float (double-precision)"))
  (bind _newhealth (`/Game/_DEV/DamageSystem/BPC_DamageSystem.Heal` (`self.BPC_DamageSystem`) Amount))
  (return _newhealth))

(fn `SetMovementSpeed`
  (params (Speed :type "/Game/_DEV/Blueprints/Enemy/AI/Enums/E_MovementSpeed Enum" :default "NewEnumerator0"))
  (returns (SpeedValue :type "Float (double-precision)"))
  (set `CharacterMovementComponent.MaxWalkSpeed` (select `/Game/_DEV/Blueprints/Enemy/AI/Enums/E_MovementSpeed` Speed :`NewEnumerator1` 250.0 :`NewEnumerator2` 500.0 :`NewEnumerator3` 500.0 :!type "Float (single-precision)") (`self.CharacterMovement`))
  (return 0.0))

(fn `TakeDamage`
  (params (DamageInfo :type "/Game/_DEV/DamageSystem/S_DamageInfo Structure"))
  (returns (WasDamaged :type Boolean))
  (bind _wasdamaged (`/Game/_DEV/DamageSystem/BPC_DamageSystem.TakeDamage` (`self.BPC_DamageSystem`) DamageInfo))
  (return _wasdamaged))

(fn `UserConstructionScript`
  (bind _bpc_damagesystem (`self.BPC_DamageSystem`))
  ;[0.01096 0.01161 0.0137] BindingDamageSystem Events
  (add `/Game/_DEV/DamageSystem/BPC_DamageSystem.OnDeath` _bpc_damagesystem (`|CreateDelegate` :!event `Death`))
  (add `/Game/_DEV/DamageSystem/BPC_DamageSystem.OnBlocked` _bpc_damagesystem (`|CreateDelegate` :!event `Blocked`))
  (add `/Game/_DEV/DamageSystem/BPC_DamageSystem.OnDamageResponse` _bpc_damagesystem (`|CreateDelegate` :!event `DamageResponse`)))