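; Base weapon actor that pulls stats, ammo, sounds and impact VFX from its DT_WeaponType row at construction and BeginPlay.
; Hit events send damage through TakeDamageMessage and play headshot or normal hit feedback on the player's crosshair widget.
; Fire and reload events play player montages and weapon animations, with HandleReload running when the reload montage completes.
; CreateFields applies radial strain and force fields to break destructible objects at a given location.
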(event `self.EnemyHit`
  (params (DamageDone :type "Float (single-precision)") (EnemyActorHit :type "Actor Object Reference") (Hit :type "HitResult Structure"))
  ;[0.7999 0.8475 1] Enemy Damage
  (message `/Game/_DEV/Interfaces/BPI_Damagable.TakeDamage` EnemyActorHit (make `/Game/_DEV/DamageSystem/S_DamageInfo` DamageDone "NewEnumerator2" "NewEnumerator1")))

(event `self.GetHitActor`
  (params (HitActor :type "Actor Object Reference"))
  (bind _wasdamaged (message `/Game/_DEV/Interfaces/BPI_Damagable.TakeDamage` HitActor (make `/Game/_DEV/DamageSystem/S_DamageInfo` 10.0 "NewEnumerator1" "NewEnumerator1")))
  (if _wasdamaged
    _))

(event `self.ShotEnemy`
  (params (bIsHeadshot :type Boolean))
  ;[0.7999 0.8475 1] Headshot and Enemy detection
  (bind _playerref (message `/Game/_DEV/Interfaces/BPI_GetCombatCharacter.GetPlayerRef` (`GameplayStatics.GetPlayerCharacter` 0)))
  (bind _wbp_stealth_game_ui (`/Game/_DEV/Blueprints/BP_CombatCharacter.WBP Stealth Game UI` _playerref)
    (:`then`
      (bind _dynamic_crosshair_w (`/Game/_DEV/UI/StealthGameUI/WBP_InGameStealth.Dynamic_Crosshair_W` _wbp_stealth_game_ui)
        (:`then`
          (if bIsHeadshot
            (`/Game/DynamicCrosshair/Blueprints/Dynamic_Crosshair_W.PlayHit` _dynamic_crosshair_w false true)
            (else
              (`/Game/DynamicCrosshair/Blueprints/Dynamic_Crosshair_W.PlayHit` _dynamic_crosshair_w false false))))
        (:`else`)))
    (:`else`)))

(event `self.CreateFields`
  (params (FieldLocation :type "Vector Structure (by ref)"))
  (bind _fieldsystem (`self.FieldSystem`))
  ;[0.7999 0.8475 1] BreakingObjects
  (`FieldSystemComponent.ApplyPhysicsField` _fieldsystem true "Field_ExternalClusterStrain" null (`RadialFalloff.SetRadialFalloff` (`self.RadialFalloff`) 1000000.0 0.8 1.0 0.0 200.0 FieldLocation "Field_FallOff_None"))
  (`FieldSystemComponent.ApplyPhysicsField` _fieldsystem true "Field_LinearForce" (`self.FieldSystemMetaDataFilter`) (`RadialVector.SetRadialVector` (`self.RadialVector`) 15000000.0 FieldLocation)))

(event `self.ReceiveBeginPlay`
  (bind _returnvalue (`|GetDataTableRow` "/Game/_DEV/DataTable/Weapon/DT_WeaponType.DT_WeaponType" (`self.WeaponName`))
    (:`then`
      (bind (_weaponname _weaponhandsocketname _weaponclass _weaponicon _weaponiconsize _weaponcrosshair _crosshairsize _lightattackmontages _lightattackmontages_2 _heavyattackmontages _heavyattackmontages_2 _comboattackmontages _isstealthweapon _takedownbehindattackermontage _takedownfrontattackermontage _takedownbehindvictimmontage _takedownfrontvictimmontage _behindtakedownhorizontaldistance _behindtakedownverticaldistance _fronttakedownhorizontaldistance _fronttakedownverticaldistance _hitsoundflesh _hitsoundwood _hitsoundmetal _ns_bloodimpactfx _cs_woodimpactfx _cs_metalimpactfx _ns_metalsparksimpactfx _weaponequipsound _currentammo _reserveammo _magazinesize _dynamiccrosshair _dynamiccrosshairsettings _bisautomatic _firerate _weaponrange _weaponreloadanimation _weaponplayerfiremontage _weaponfireanimation _weaponfiresound _weaponplayerreloadmontage _emptyclipsound _gunwoodhitvfx _gunmetalhitvfx _gunenemyhitniagaravfx _basedamage _headshotmultiplier _limbmultiplier _spreadhipdeg _spreadadsdeg _recoilpitchmin _recoilpitchmax _recoilyawmin _recoilyawmax _recoilcamerashake _tracerfx) (break `/Game/_DEV/DataTable/Weapon/S_WeaponType` _returnvalue))
      (set `self.WeaponID` _weaponname)
      (set `self.HitEnemySound` _hitsoundflesh)
      (set `self.HitEnvironmentSoundWood` _hitsoundwood)
      (set `self.HitEnvironmentSoundMetal` _hitsoundmetal)
      (set `self.EnemyHitVFX` null)
      (set `self.EnemyHitNiagaraVFX` _ns_bloodimpactfx)
      (set `self.WoodHitVFX` _cs_woodimpactfx)
      (set `self.WoodHitNiagaraVFX` null)
      (set `self.MetalHitVFX` _cs_metalimpactfx)
      (set `self.MetalHitNiagaraVFX` _ns_metalsparksimpactfx)
      (set `self.CurrentAmmo` _currentammo)
      (set `self.ReserveAmmo` _reserveammo)
      (set `self.MagazineSize` _magazinesize)
      (set `self.FireRate` _firerate)
      (set `self.WeaponRange` _weaponrange)
      (set `self.EmptyClipSound` _emptyclipsound)
      (set `self.GunWoodHitVFX` _gunwoodhitvfx)
      (set `self.GunMetalHitVFX` _gunmetalhitvfx)
      (set `self.GunEnemyHitNiagaraVFX` _gunenemyhitniagaravfx)
      (set `self.BaseDamage` _basedamage)
      (set `self.HeadshotMultiplier` _headshotmultiplier)
      (set `self.LimbMultiplier` _limbmultiplier)
      (set `self.DamageTypeClass` "/Script/Engine.DamageType")
      (set `self.SpreadHipDeg` _spreadhipdeg)
      (set `self.SpreadADSDeg` _spreadadsdeg)
      (set `self.RecoilPitchMin` _recoilpitchmin)
      (set `self.RecoilPitchMax` _recoilpitchmax)
      (set `self.RecoilYawMin` _recoilyawmin)
      (set `self.RecoilYawMax` _recoilyawmax)
      (set `self.RecoilCameraShake` _recoilcamerashake)
      (set `self.TracerFX` _tracerfx)
      (set `self.bIsAutomatic` _bisautomatic)
      (set `self.WeaponFireSound` _weaponfiresound))))

(event `self.PlayFireEffects`
  ;[0.7499 0.7945 0.9375] Play Player Fire Montage
  (bind _playerref (message `/Game/_DEV/Interfaces/BPI_GetCombatCharacter.GetPlayerRef` (`self.GetOwner`)))
  (bind (_weaponname _weaponhandsocketname _weaponclass _weaponicon _weaponiconsize _weaponcrosshair _crosshairsize _lightattackmontages _lightattackmontages_2 _heavyattackmontages _heavyattackmontages_2 _comboattackmontages _isstealthweapon _takedownbehindattackermontage _takedownfrontattackermontage _takedownbehindvictimmontage _takedownfrontvictimmontage _behindtakedownhorizontaldistance _behindtakedownverticaldistance _fronttakedownhorizontaldistance _fronttakedownverticaldistance _hitsoundflesh _hitsoundwood _hitsoundmetal _ns_bloodimpactfx _cs_woodimpactfx _cs_metalimpactfx _ns_metalsparksimpactfx _weaponequipsound _currentammo _reserveammo _magazinesize _dynamiccrosshair _dynamiccrosshairsettings _bisautomatic _firerate _weaponrange _weaponreloadanimation _weaponplayerfiremontage _weaponfireanimation _weaponfiresound _weaponplayerreloadmontage _emptyclipsound _gunwoodhitvfx _gunmetalhitvfx _gunenemyhitniagaravfx _basedamage _headshotmultiplier _limbmultiplier _spreadhipdeg _spreadadsdeg _recoilpitchmin _recoilpitchmax _recoilyawmin _recoilyawmax _recoilcamerashake _tracerfx) (break `/Game/_DEV/DataTable/Weapon/S_WeaponType` (stale `self.ReceiveBeginPlay` _returnvalue)))
  (`|PlayMontage` (`Character.Mesh` _playerref) _weaponplayerfiremontage
    (:`then`
      (`GameplayStatics.PlaySoundAtLocation` (`self.WeaponFireSound`) (`self.K2_GetActorLocation`) (struct) 1.0 1.0 0.0 null null null null)
      (`SkeletalMeshComponent.PlayAnimation` (`self.Mesh`) _weaponfireanimation false))))

(event `self.PlayReloadEffects`
  ;[0.7999 0.8475 1] Reload
  (set `self.bIsReloading` true)
  (bind _playerref (message `/Game/_DEV/Interfaces/BPI_GetCombatCharacter.GetPlayerRef` (`self.GetOwner`)))
  (bind (_weaponname _weaponhandsocketname _weaponclass _weaponicon _weaponiconsize _weaponcrosshair _crosshairsize _lightattackmontages _lightattackmontages_2 _heavyattackmontages _heavyattackmontages_2 _comboattackmontages _isstealthweapon _takedownbehindattackermontage _takedownfrontattackermontage _takedownbehindvictimmontage _takedownfrontvictimmontage _behindtakedownhorizontaldistance _behindtakedownverticaldistance _fronttakedownhorizontaldistance _fronttakedownverticaldistance _hitsoundflesh _hitsoundwood _hitsoundmetal _ns_bloodimpactfx _cs_woodimpactfx _cs_metalimpactfx _ns_metalsparksimpactfx _weaponequipsound _currentammo _reserveammo _magazinesize _dynamiccrosshair _dynamiccrosshairsettings _bisautomatic _firerate _weaponrange _weaponreloadanimation _weaponplayerfiremontage _weaponfireanimation _weaponfiresound _weaponplayerreloadmontage _emptyclipsound _gunwoodhitvfx _gunmetalhitvfx _gunenemyhitniagaravfx _basedamage _headshotmultiplier _limbmultiplier _spreadhipdeg _spreadadsdeg _recoilpitchmin _recoilpitchmax _recoilyawmin _recoilyawmax _recoilcamerashake _tracerfx) (break `/Game/_DEV/DataTable/Weapon/S_WeaponType` (stale `self.ReceiveBeginPlay` _returnvalue)))
  (`|PlayMontage` (`Character.Mesh` _playerref) _weaponplayerreloadmontage
    (:`then`
      (`SkeletalMeshComponent.PlayAnimation` (`self.Mesh`) _weaponreloadanimation false))
    (:`OnCompleted`
      (`self.HandleReload`)
      (set `self.bIsReloading` false))))

(fn `UserConstructionScript`
  (bind _returnvalue (`|GetDataTableRow` "/Game/_DEV/DataTable/Weapon/DT_WeaponType.DT_WeaponType" (`self.WeaponName`))
    (:`then`
      (bind (_weaponname _weaponhandsocketname _weaponclass _weaponicon _weaponiconsize _weaponcrosshair _crosshairsize _lightattackmontages _lightattackmontages_2 _heavyattackmontages _heavyattackmontages_2 _comboattackmontages _isstealthweapon _takedownbehindattackermontage _takedownfrontattackermontage _takedownbehindvictimmontage _takedownfrontvictimmontage _behindtakedownhorizontaldistance _behindtakedownverticaldistance _fronttakedownhorizontaldistance _fronttakedownverticaldistance _hitsoundflesh _hitsoundwood _hitsoundmetal _ns_bloodimpactfx _cs_woodimpactfx _cs_metalimpactfx _ns_metalsparksimpactfx _weaponequipsound _currentammo _reserveammo _magazinesize _dynamiccrosshair _dynamiccrosshairsettings _bisautomatic _firerate _weaponrange _weaponreloadanimation _weaponplayerfiremontage _weaponfireanimation _weaponfiresound _weaponplayerreloadmontage _emptyclipsound _gunwoodhitvfx _gunmetalhitvfx _gunenemyhitniagaravfx _basedamage _headshotmultiplier _limbmultiplier _spreadhipdeg _spreadadsdeg _recoilpitchmin _recoilpitchmax _recoilyawmin _recoilyawmax _recoilcamerashake _tracerfx) (break `/Game/_DEV/DataTable/Weapon/S_WeaponType` _returnvalue))
      (set `self.HitEnemySound` _hitsoundflesh)
      (set `self.HitEnvironmentSoundWood` _hitsoundwood)
      (set `self.HitEnvironmentSoundMetal` _hitsoundmetal)
      (set `self.EnemyHitVFX` null)
      (set `self.EnemyHitNiagaraVFX` _ns_bloodimpactfx)
      (set `self.WoodHitVFX` _cs_woodimpactfx)
      (set `self.WoodHitNiagaraVFX` null)
      (set `self.MetalHitVFX` _cs_metalimpactfx)
      (set `self.MetalHitNiagaraVFX` _ns_metalsparksimpactfx)
      (set `self.CurrentAmmo` _currentammo)
      (set `self.ReserveAmmo` _reserveammo)
      (set `self.MagazineSize` _magazinesize)
      (set `self.FireRate` _firerate)
      (set `self.WeaponRange` _weaponrange)
      (set `self.EmptyClipSound` _emptyclipsound)
      (set `self.GunWoodHitVFX` _gunwoodhitvfx)
      (set `self.GunMetalHitVFX` _gunmetalhitvfx)
      (set `self.GunEnemyHitNiagaraVFX` _gunenemyhitniagaravfx)
      (set `self.BaseDamage` _basedamage)
      (set `self.HeadshotMultiplier` _headshotmultiplier)
      (set `self.LimbMultiplier` _limbmultiplier)
      (set `self.DamageTypeClass` "/Script/Engine.DamageType")
      (set `self.SpreadHipDeg` _spreadhipdeg)
      (set `self.SpreadADSDeg` _spreadadsdeg)
      (set `self.RecoilPitchMin` _recoilpitchmin)
      (set `self.RecoilPitchMax` _recoilpitchmax)
      (set `self.RecoilYawMin` _recoilyawmin)
      (set `self.RecoilYawMax` _recoilyawmax)
      (set `self.RecoilCameraShake` _recoilcamerashake)
      (set `self.TracerFX` _tracerfx))))